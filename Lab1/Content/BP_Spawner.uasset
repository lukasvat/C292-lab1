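; BP_Spawner is a spawner Blueprint that spawns one actor when play begins.
; BeginPlay takes the transform of an entry in the SpwnPositions array, using a random index whose range is zero to zero, so the first entry is always chosen.
; A disconnected loop that would spawn an actor at every position remains in the graph but never runs.
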(event EventBeginPlay
  (Game|SpawnActorfromClass 0 (Transformation|GetActorTransform (Utilities|Array|Get(acopy) (Variables|Default|GetSpwn%20Positions) (Math|Random|RandomIntegerinRange 0 0))) "Undefined" "MultiplyWithRoot" 0))

(fn ConstructionScript)